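; GA_HitReact is a Gameplay Ability that runs an avatar's hit reaction.
; On activation it applies GE_HitReact to the owner and stores the handle, then gets a montage through CombatInterface.
; It ends when that montage completes, is interrupted or is cancelled, or after a short delay if no montage is valid.
; Ending removes the effect by handle; an avatar lacking CombatInterface never reaches EndAbility here.
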(event `self.K2_ActivateAbility`
  (bind _returnvalue (`self.GetAvatarActorFromActorInfo`))
  (`|ExecutionSequence`
    (:`then_0`
      (bind _returnvalue_2 (`self.BP_ApplyGameplayEffectToOwner` "/Game/Blueprints/AbilitySystem/GameplayEffect/GE_HitReact.GE_HitReact_C"))
      (set `self.GEHandle` _returnvalue_2)
      (if (`KismetSystemLibrary.DoesImplementInterface` _returnvalue "/Script/Aura.CombatInterface")
        (bind _returnvalue_3 (message `CombatInterface.GetHitReactMontage` _returnvalue))
        (`/Engine/EditorBlueprintResources/StandardMacros.IsValid` _returnvalue_3
          (:`Is Valid`
            (`AbilityTask_PlayMontageAndWait.CreatePlayMontageAndWaitProxy` "None" _returnvalue_3
              (:`OnCompleted`
                _)
              (:`OnInterrupted`
                _)
              (:`OnCancelled`
                _)))
          (:`Is Not Valid`
            (`KismetSystemLibrary.Delay` 0.5)))
        (`self.K2_EndAbility`)))))

(event `self.K2_OnEndAbility`
  (params (bWasCancelled :type Boolean))
  (`self.BP_RemoveGameplayEffectFromOwnerWithHandle` (`self.GEHandle`)))