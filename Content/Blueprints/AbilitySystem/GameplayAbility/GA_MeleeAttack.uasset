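; Enemy melee attack gameplay ability that faces the avatar toward its combat target and plays a random tagged attack montage.
; The montage's gameplay event triggers a small radius check at the tag's combat socket, damaging live players found there.
; Any hit fires one MeleeAttackImpact GameplayCue carrying the montage's data tag, replacing the disconnected sound and blood-effect nodes.
; Avatars lacking EnemyInterface do nothing, and that path never calls EndAbility.
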(event `self.K2_ActivateAbility`
  (bind _returnvalue (`self.GetAvatarActorFromActorInfo`))
  (bind _returnvalue_2 (`self.GetAvatarActorFromActorInfo`))
  (bind _returnvalue_3 (`self.GetAvatarActorFromActorInfo`))
  (bind _attacktaggedmontage_montagedatatag (break `TaggedMontage` (`self.AttackTaggedMontage`)))
  (set `self.HasHitTarget` false)
  (if (`KismetSystemLibrary.DoesImplementInterface` _returnvalue_3 "/Script/Aura.EnemyInterface")
    (`|ExecutionSequence`
      (:`then_0`
        (bind _returnvalue_4 (message `EnemyInterface.GetCombatTarget` _returnvalue_2))
        (bind _output_get (set `self.CombatTarget` _returnvalue_2))
        (message `CombatInterface.UpdateFacingTarget` _output_get (`Actor.K2_GetActorLocation` _returnvalue_4)))
      (:`then_1`
        (bind _returnvalue_5 (message `CombatInterface.GetAttackMontages` _returnvalue_3))
        (bind _output_get_2 (set `self.AttackTaggedMontage` (`KismetArrayLibrary.Array_Random` _returnvalue_5)))
        (bind (_montagedatatag _montageinnertag _montage) (break `TaggedMontage` _output_get_2))
        (`AbilityTask_PlayMontageAndWait.CreatePlayMontageAndWaitProxy` "None" _montage
          (:`then`
            (`AbilityTask_WaitGameplayEvent.WaitGameplayEvent` _montageinnertag null
              (:`EventReceived`
                (bind _returnvalue_6 (message `CombatInterface.GetCombatSocketLocation` _returnvalue _montageinnertag))
                (bind _output_get_3 (set `self.CombatLocation` _returnvalue_6))
                (bind _outactors (`AuraAbilitySystemLibrary.GetLivePlayersWithinRadius` (`|MakeArray` _returnvalue) _output_get_3 20.0))
                (for _array_element _outactors
                  (`self.CauseDamage` _array_element)
                  (set `self.HasHitTarget` true)
                  (bind _returnvalue_7 (message `CombatInterface.GetBloodEffect` _array_element)))
                (if (`self.HasHitTarget`)
                  (`self.K2_ExecuteGameplayCueWithParams` (struct :`TagName` "GameplayCue.MeleeAttackImpact") (`AbilitySystemBlueprintLibrary.MakeGameplayCueParameters` 0.0 0.0 (struct) (struct) (struct) (`BlueprintGameplayTagLibrary.MakeGameplayTagContainerFromTag` _attacktaggedmontage_montagedatatag) (struct) (`self.CombatLocation`) (0.0 0.0 0.0) null (`self.GetAvatarActorFromActorInfo`) (`self.CombatTarget`))))
                (`self.K2_EndAbility`))))
          (:`OnCompleted`
            (`self.K2_EndAbility` :!label _label))
          (:`OnInterrupted`
            (goto _label))
          (:`OnCancelled`
            (goto _label)))))))