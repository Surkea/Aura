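; Fire Bolt gameplay ability that launches a projectile at the location under the mouse cursor.
; An ability task supplies mouse target data, then the avatar turns toward that point through CombatInterface and plays a random attack montage from that interface.
; A gameplay event matching a randomly picked montage tag triggers the projectile spawn, and the ability ends after a short delay.
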(event `self.K2_ActivateAbility`
  (bind _returnvalue (`self.GetAvatarActorFromActorInfo`))
  (bind (_asynctaskproxy _datahandle) (`GetTargetDataUnderMouse.CreateProxy`)
    (:`OnGetMouseTargetData`
      (set `self.ProjectileTargetLocation` (`.Location` (`GameplayStatics.BreakHitResult` (`AbilitySystemBlueprintLibrary.GetHitResultFromTargetData` _datahandle))))
      (if (`KismetSystemLibrary.DoesImplementInterface` _returnvalue "/Script/Aura.CombatInterface")
        (message `CombatInterface.UpdateFacingTarget` _returnvalue (`self.ProjectileTargetLocation`))
        (bind _returnvalue_2 (message `CombatInterface.GetAttackMontages` (`self.GetAvatarActorFromActorInfo`)))
        (bind _outitem (`KismetArrayLibrary.Array_Random` _returnvalue_2))
        (`AbilityTask_PlayMontageAndWait.CreatePlayMontageAndWaitProxy` "None" (break `TaggedMontage` _outitem)
          (:`then`
            (`AbilityTask_WaitGameplayEvent.WaitGameplayEvent` (`.MontageTag` (break `TaggedMontage` _outitem)) null
              (:`EventReceived`
                (`self.SpawnProjectile` (`self.ProjectileTargetLocation`))
                (`KismetSystemLibrary.Delay` 0.5)
                (`self.K2_EndAbility`)))))))))