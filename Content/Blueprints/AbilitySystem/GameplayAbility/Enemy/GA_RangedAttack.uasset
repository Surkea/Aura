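; Enemy ranged attack gameplay ability that fires a projectile at the avatar's current combat target.
; On activation it caches the target's location and turns the avatar to face it, both through enemy interface messages.
; It plays a random tagged attack montage, waits for the gameplay event matching that montage's tag, spawns the projectile, then ends shortly after.
; The ability also ends when the montage completes, is interrupted or is cancelled.
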(event `self.K2_ActivateAbility`
  (bind _returnvalue (`self.GetAvatarActorFromActorInfo`))
  (bind _returnvalue_2 (`self.GetAvatarActorFromActorInfo`))
  (if (`KismetSystemLibrary.DoesImplementInterface` _returnvalue_2 "/Script/Aura.EnemyInterface")
    (`|ExecutionSequence`
      (:`then_0`
        (bind _returnvalue_3 (message `EnemyInterface.GetCombatTarget` _returnvalue))
        (bind _output_get (set `self.AttackTargetLocation` (`Actor.K2_GetActorLocation` _returnvalue_3)))
        (message `CombatInterface.UpdateFacingTarget` _returnvalue _output_get))
      (:`then_1`
        (bind _returnvalue_4 (message `CombatInterface.GetAttackMontages` _returnvalue_2))
        (bind _output_get_2 (set `self.AttackTaggedMontage` (`KismetArrayLibrary.Array_Random` _returnvalue_4)))
        (bind (_montage _montagetag) (break `TaggedMontage` _output_get_2))
        (`AbilityTask_PlayMontageAndWait.CreatePlayMontageAndWaitProxy` "None" _montage
          (:`then`
            (`AbilityTask_WaitGameplayEvent.WaitGameplayEvent` _montagetag null
              (:`EventReceived`
                (`self.SpawnProjectile` (`self.AttackTargetLocation`))
                (`KismetSystemLibrary.Delay` 0.5)
                (`self.K2_EndAbility`))))
          (:`OnCompleted`
            (`self.K2_EndAbility` :!label _label))
          (:`OnInterrupted`
            (goto _label))
          (:`OnCancelled`
            (goto _label)))))))